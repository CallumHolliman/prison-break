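; BP_Enemy_Random is an enemy that takes damage and ends the player's run on contact.
; Damage lowers its clamped health, updates an overhead health bar widget and destroys the actor at zero.
; A sphere trigger shows the bar while an actor tagged Player is inside.
; A box trigger calls IsCaughtMessage on the player character when touched by the player.
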(event OnComponentBeginOverlap(Sphere)
  (params (OverlappedComponent :type Primitive%20Component%20Object%20Reference) (OtherActor :type Actor%20Object%20Reference) (OtherComp :type Primitive%20Component%20Object%20Reference) (OtherBodyIndex :type Integer) (bFromSweep :type Boolean) (SweepResult :type Hit%20Result%20Structure%20%28by%20ref%29))
  ;[1 1 1] show health bar if in radius
  (if (Actor|ActorHasTag OtherActor "Player")
    (Rendering|SetVisibility (Variables|Default|GetWidget) true false)))

(event OnComponentEndOverlap(Sphere)
  (params (OverlappedComponent :type Primitive%20Component%20Object%20Reference) (OtherActor :type Actor%20Object%20Reference) (OtherComp :type Primitive%20Component%20Object%20Reference) (OtherBodyIndex :type Integer))
  ;[1 1 1] show health bar if in radius
  (if (Actor|ActorHasTag OtherActor "Player")
    (Rendering|SetVisibility (Variables|Default|GetWidget) false false)))

(event OnComponentBeginOverlap(Box)
  (params (OverlappedComponent :type Primitive%20Component%20Object%20Reference) (OtherActor :type Actor%20Object%20Reference) (OtherComp :type Primitive%20Component%20Object%20Reference) (OtherBodyIndex :type Integer) (bFromSweep :type Boolean) (SweepResult :type Hit%20Result%20Structure%20%28by%20ref%29))
  ;[1 1 1] if touching player, end game
  (if (Actor|ActorHasTag OtherActor "Player")
    (Class|BPIPlayerCaught|IsCaught(Message) (Game|GetPlayerCharacter 0))))

(event EventBeginPlay
  ;[1 1 1] set health bar
  (bind _asoverhead_health_bar (Utilities|Casting|CastToOverheadHealthBar (UserInterface|GetUserWidgetObject (Variables|Default|GetWidget))))
  (Variables|Default|SetHealthWidgetRef _asoverhead_health_bar))

(event Game|Damage|EventAnyDamage
  (params (Damage :type Float%20%28single-precision%29) (DamageType :type Damage%20Type%20Object%20Reference) (InstigatedBy :type Controller%20Object%20Reference) (DamageCauser :type Actor%20Object%20Reference))
  ;[1 1 1] damage calculation/death
  (bind _output_get (Variables|Default|SetHealth (Math|Float|Clamp(Float) (- (Variables|Default|GetHealth) Damage) 0.0 1e+02)))
  (Variables|/Game/Widgets/OverheadHealthBar.OverheadHealthBar_C|SetHealth (Variables|Default|GetHealthWidgetRef) _output_get)
  (CallFunction|UpdateHealthBar _output_get)
  (if (== _output_get 0.0)
    (Actor|DestroyActor)))

(fn ConstructionScript)